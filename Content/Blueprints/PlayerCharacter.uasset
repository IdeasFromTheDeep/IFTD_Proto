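; Player character for a twin-stick shooter, with left-stick movement along world axes and right-stick aiming that fires automatically.
; Right-stick deflection beyond a dead zone sets control rotation and pulls the rifle trigger, otherwise releasing it.
; BeginPlay spawns the rifle onto TempGun and records the spawn transform in TwinStickMode.
; AffectHealth updates health and, on death, requests a respawn before destroying rifle and character.
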(event `InputAxis|MoveUp`
  (params (AxisValue :type "Float (single-precision)"))
  ;[1 1 1] Left Stick (Movement)
  (`self.AddMovementInput` (1.0 0.0 0.0) AxisValue))

(event `InputAxis|LookUp`
  (params (AxisValue :type "Float (single-precision)"))
  (bind _rifle (`self.Rifle`))
  ;[1 1 1] Right Stick (Camera/Gun Control)
  (bind _returnvalue (`KismetMathLibrary.MakeVector` AxisValue (stale `InputAxis|LookRight` AxisValue)))
  (if (> (`KismetMathLibrary.VSize` _returnvalue) 0.25) :!label _label
    (`Controller.SetControlRotation` (`self.GetController`) (`KismetMathLibrary.Conv_VectorToRotator` _returnvalue))
    (`/Game/Blueprints/PlayeRifle.PullTrigger` _rifle)
    (else
      (`/Game/Blueprints/PlayeRifle.Release Trigger` _rifle))))

(event `InputAxis|LookRight`
  (params (AxisValue :type "Float (single-precision)"))
  ;[1 1 1] Right Stick (Camera/Gun Control)
  (goto _label))

(event `InputAxis|MoveRight`
  (params (AxisValue :type "Float (single-precision)"))
  ;[1 1 1] Left Stick (Movement)
  (`self.AddMovementInput` (0.0 1.0 0.0) AxisValue))

(event `self.ReceiveBeginPlay`
  (bind _tempgun (`self.TempGun`))
  ;[1 1 1] Spawn Hero and Rifle
  (`|ExecutionSequence`
    (:`then_0`
      (bind _returnvalue (`|SpawnActorFromClass` "/Game/Blueprints/PlayeRifle.PlayeRifle_C" (`SceneComponent.K2_GetComponentToWorld` _tempgun) "Undefined" "OverrideRootScale"))
      (bind _output_get (set `self.Rifle` _returnvalue))
      (`self.K2_AttachToComponent` _output_get _tempgun "None" "SnapToTarget" "SnapToTarget" "KeepRelative" true))
    (:`then_1`
      (bind _astwin_stick_mode (cast `/Game/Blueprints/TwinStickMode` (`GameplayStatics.GetGameMode`)))
      (bind _output_get_2 (set `self.TSGameMode` _astwin_stick_mode))
      (set `/Game/Blueprints/TwinStickMode.PlayerSpawnTransform` (`self.GetTransform`) _output_get_2))))

(event `/Game/Blueprints/iDamageable.AffectHealth`
  (params (Delta :type "Float (single-precision)"))
  ;[1 1 1] Handle Damage
  (`self.CalculateHealth` Delta)
  (if (`self.isDead`)
    (`/Game/Blueprints/TwinStickMode.RespawnPlayer` (`self.TSGameMode`))
    (`self.K2_DestroyActor` (`self.Rifle`))
    (`self.K2_DestroyActor` self)))

(fn `UserConstructionScript`)