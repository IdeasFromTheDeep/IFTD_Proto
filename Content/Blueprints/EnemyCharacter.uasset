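; Enemy character that deals periodic contact damage to the player and can be killed.
; Overlapping a PlayerCharacter starts a looping timer, paced by attacks per second, that damages the hero through AffectHealth until the overlap ends.
; Its own AffectHealth recalculates health and, on death, disables pawn and world-dynamic collision, detaches the controller and destroys the actor after a delay.
; The construction script tints the body through a dynamic material instance.
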(event `/Game/Blueprints/iDamageable.AffectHealth`
  (params (Delta :type "Float (single-precision)"))
  (bind _capsulecomponent (`self.CapsuleComponent`))
  ;[1 1 1] Handle Damage
  (`self.CalculateHealth` Delta)
  (if (`self.isDead`)
    (`PrimitiveComponent.SetCollisionResponseToChannel` _capsulecomponent "ECC_WorldDynamic" "ECR_Ignore")
    (`PrimitiveComponent.SetCollisionResponseToChannel` _capsulecomponent "ECC_Pawn" "ECR_Ignore")
    (`self.DetachFromControllerPendingDestroy`)
    (`KismetSystemLibrary.Delay` 3.0)
    (`self.K2_DestroyActor`)))

(event `self.ReceiveActorBeginOverlap`
  (params (OtherActor :type "Actor Object Reference"))
  ;[1 1 1] Detect Collision
  (bind _asplayer_character (cast `/Game/Blueprints/PlayerCharacter` OtherActor))
  (set `self.Hero` _asplayer_character)
  (`KismetSystemLibrary.K2_SetTimer` null "DamageHero" (/ 1.0 (`self.AttacksPerSecond`)) true))

(event `self.ReceiveActorEndOverlap`
  (params (OtherActor :type "Actor Object Reference"))
  ;[1 1 1] Stop Taking Damage
  (if (== OtherActor (`self.Hero`))
    (`KismetSystemLibrary.K2_ClearTimer` null "DamageHero")))

(event `DamageHero`
  ;[1 1 1] TakeDamage
  (`/Game/Blueprints/PlayerCharacter.AffectHealth` (`self.Hero`) (`self.Damage`)))

(fn `UserConstructionScript`
  (bind _returnvalue (`PrimitiveComponent.CreateDynamicMaterialInstance` (`self.Mesh`) 0 "/Game/AnimationAssets/UE4_Mannequin/Materials/M_UE4Man_Body.M_UE4Man_Body"))
  (bind _output_get (set `self.DynaMat` _returnvalue))
  (`MaterialInstanceDynamic.SetVectorParameterValue` _output_get "BodyColor" (`self.EnemyColor`)))