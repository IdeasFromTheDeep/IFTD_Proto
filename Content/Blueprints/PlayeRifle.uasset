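; Player rifle Blueprint that provides automatic fire while the trigger is held.
; PullTrigger passes through a DoOnce to fire immediately, then starts a looping timer that calls Fire at the RoundsPerSecond rate.
; Fire spawns a PlayerProjectile at the ProjectileSpawnPoint transform.
; ReleaseTrigger clears the timer and resets the DoOnce, so the next pull fires at once with no cooldown between pulls.
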(event `Fire`
  ;[1 1 1] SpawnProjectile (Fire)
  (`|SpawnActorFromClass` "/Game/Blueprints/PlayerProjectile.PlayerProjectile_C" (`SceneComponent.K2_GetComponentToWorld` (`self.ProjectileSpawnPoint`)) "Undefined" "OverrideRootScale"))

(event `PullTrigger`
  ;[1 1 1] TirggerPull Timer
  (`/Engine/EditorBlueprintResources/StandardMacros.DoOnce` false :!label _label
    (:`Completed`
      (`self.Fire`)
      (`KismetSystemLibrary.K2_SetTimer` null "Fire" (/ 1.0 (`self.RoundsPerSecond`)) true))))

(event `Release Trigger`
  ;[1 1 1] TirggerPull Timer
  (`KismetSystemLibrary.K2_ClearTimer` null "Fire")
  (goto _label :!via `Reset`))

(fn `UserConstructionScript`)